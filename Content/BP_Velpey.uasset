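; Velpey character Blueprint that drives SDF face shading from the directional light's yaw relative to the head socket.
; The construction script swaps the face material for a dynamic instance and starts a fast looping timer, apparently for Update.
; Update maps dot and cross products of both forward vectors through a curve into SDF_Location.
; When no light is cached, it grabs the first DirectionalLight and applies an older curve-free formula.
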(event `Update`
  (bind _newfacematerial (`self.newFaceMaterial`))
  (bind _curve (`self.Curve`))
  (bind (_returnvalue_roll _returnvalue_pitch _returnvalue_yaw) (`KismetMathLibrary.BreakRotator` (`self.K2_GetActorRotation` (`self.DirectionLight`))))
  (bind _returnvalue (`KismetMathLibrary.GetForwardVector` (`SceneComponent.GetSocketRotation` (`self.SKM_Velpey`) (`self.HeadSocketName`))))
  (bind _returnvalue_2 (`KismetMathLibrary.GetForwardVector` (`KismetMathLibrary.MakeRotator` 0.0 0.0 _returnvalue_yaw)))
  (bind (_returnvalue_x _returnvalue_y _returnvalue_z) (`KismetMathLibrary.BreakVector` (`KismetMathLibrary.Cross_VectorVector` _returnvalue_2 _returnvalue)))
  (bind _returnvalue_3 (`KismetMathLibrary.Dot_VectorVector` _returnvalue_2 _returnvalue))
  (`/Engine/EditorBlueprintResources/StandardMacros.IsValid` (`self.newFaceMaterial`)
    (:`Is Valid`
      (`/Engine/EditorBlueprintResources/StandardMacros.IsValid` (`self.DirectionLight`)
        (:`Is Valid`
          ;[1 1 1] New
          (if (<= _returnvalue_3 0.0)
            (`MaterialInstanceDynamic.SetScalarParameterValue` (`self.newFaceMaterial`) "SDF_Location" (`CurveFloat.GetFloatValue` _curve (+ (* _returnvalue_z -0.5) 0.5)))
            (else
              (`MaterialInstanceDynamic.SetScalarParameterValue` (`self.newFaceMaterial`) "SDF_Location" (`CurveFloat.GetFloatValue` _curve (- (/ _returnvalue_z 2.0) 0.5))))))
        (:`Is Not Valid`
          (bind _outactors (`GameplayStatics.GetAllActorsOfClass` "/Script/Engine.DirectionalLight"))
          (set `self.DirectionLight` (`|GetArrayItem` _outactors))
          ;[1 1 1] Old
          (if (>= _returnvalue_z 0.0)
            (`MaterialInstanceDynamic.SetScalarParameterValue` (`self.newFaceMaterial`) "SDF_Location" (/ _returnvalue_3 -2.0))
            (elif (< _returnvalue_3 0.0)
              (`MaterialInstanceDynamic.SetScalarParameterValue` _newfacematerial "SDF_Location" (+ (/ _returnvalue_3 2.0) 1.0))
              (else
                (`MaterialInstanceDynamic.SetScalarParameterValue` _newfacematerial "SDF_Location" (- (/ _returnvalue_3 2.0) 1.0))))))))))

(fn `UserConstructionScript`
  (`/Engine/EditorBlueprintResources/StandardMacros.IsValid` (`self.FaceMaterial`)
    (:`Is Valid`
      (bind _returnvalue (`KismetMaterialLibrary.CreateDynamicMaterialInstance` (`self.FaceMaterial`)))
      (bind _output_get (set `self.newFaceMaterial` _returnvalue))
      (`PrimitiveComponent.SetMaterial` (`self.SKM_Velpey`) (`KismetArrayLibrary.Array_Find` (`MeshComponent.GetMaterials` (`self.SKM_Velpey`)) (`self.FaceMaterial`)) _output_get)
      (`KismetSystemLibrary.K2_SetTimerDelegate` (`|CreateDelegate` :!event `Update`) 0.01 true))))